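; Nest interaction actor that lets the player enter and exit a nest while overlapping it, then advance to the next story scene.
; Tick polls externally set press flags; while nested, it pins the shrunken player at an Arrow positioned by the construction script and spawns a TextRenderActor every frame.
; Continuing stream-loads NextScene, repositions the player and unloads CurrentScene.
; Text-update and people-count loops are unwired.
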(event `self.ReceiveBeginPlay`)

(event `self.ReceiveActorBeginOverlap`
  (params (OtherActor :type "Actor Object Reference"))
  (set `self.IsInside` (`self.ActorHasTag` OtherActor "Player")))

(event `self.ReceiveActorEndOverlap`
  (params (OtherActor :type "Actor Object Reference"))
  (set `self.IsInside` false))

(event `self.ReceiveTick`
  (params (DeltaSeconds :type "Float (single-precision)"))
  (bind _returnvalue (`GameplayStatics.GetPlayerCharacter` 0))
  (bind _returnvalue_2 (`GameplayStatics.GetPlayerCharacter` 0))
  (bind _arrow (`self.Arrow`))
  (bind _returnvalue_location (`KismetMathLibrary.BreakTransform` (`SceneComponent.K2_GetComponentToWorld` (`self.Arrow`))))
  (bind (_returnvalue_location_2 _returnvalue_rotation) (`KismetMathLibrary.BreakTransform` (`SceneComponent.K2_GetComponentToWorld` (`Character.CapsuleComponent` (`GameplayStatics.GetPlayerCharacter` 0)))))
  (`self.EnterNest`)
  (`self.ExitNest`)
  (if (`self.InNest`)
    (`SceneComponent.K2_SetWorldTransform` (`Actor.RootComponent` _returnvalue_2) (`KismetMathLibrary.MakeTransform` _returnvalue_location _returnvalue_rotation (0.2 0.2 0.2)) false false)
    (if (== _returnvalue_2 _returnvalue)
      (set `MovementComponent.Velocity` (0.0 0.0 0.0) (`Character.CharacterMovement` _returnvalue))
      (set `self.InNest` true)
      (`|SpawnActorFromClass` "/Script/Engine.TextRenderActor" (`SceneComponent.K2_GetComponentToWorld` (`self.Arrow`)) "Undefined" "MultiplyWithRoot" null null)
      (`self.ContinueStory`)
      (if (`self.Continue`)
        (`GameplayStatics.LoadStreamLevel` (`KismetStringLibrary.Conv_StringToName` (`self.NextScene`)) true)
        (`self.K2_SetActorLocationAndRotation` (`GameplayStatics.GetPlayerCharacter` 0) (`SceneComponent.K2_GetComponentLocation` _arrow) (`SceneComponent.K2_GetComponentRotation` _arrow) false false)
        (`GameplayStatics.UnloadStreamLevel` (`KismetStringLibrary.Conv_StringToName` (`self.CurrentScene`)))))))

(event `EnterNest`
  (if (and (`self.PressingToEnter`) (`self.IsInside`) (not (`self.InNest`)))
    (set `self.InNest` true)))

(event `ExitNest`
  (if (and (`self.PressingToExit`) (`self.IsInside`) (`self.InNest`) (not (`self.PlayingStory`)))
    (set `self.InNest` false)))

(event `ContinueStory`
  (if (and (`self.IsInside`) (`self.InNest`) (`self.PressingToNextScene`))
    (set `self.Continue` true)
    (else
      (set `self.Continue` false))))

(fn `UserConstructionScript`
  (`SceneComponent.K2_SetRelativeTransform` (`self.Arrow`) (`self.Teleport Location`) false false))