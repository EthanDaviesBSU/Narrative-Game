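; BP_FadeGame is an ending-choice actor that lets the player finish the game in a good or bad ending zone.
; The Good and Bad overlap components show their prompt widgets and set inside flags, whose names are swapped relative to the zones.
; Tick checks PressingToEnd, which is not set here, then fades the camera white for Good or black for Bad and opens MainMenuMap after a delay.
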(event `self.ReceiveBeginPlay`
  (bind _returnvalue (`|CreateWidget` "/Game/UI/PromptGoodEnding.PromptGoodEnding_C"))
  (set `self.GoodEnding` _returnvalue)
  (bind _returnvalue_2 (`|CreateWidget` "/Game/UI/PromptBadEnding.PromptBadEnding_C"))
  (set `self.BadEnding` _returnvalue_2))

(event `self.Bad.OnComponentBeginOverlap`
  (params (OverlappedComponent :type "PrimitiveComponent Object Reference") (OtherActor :type "Actor Object Reference") (OtherComp :type "PrimitiveComponent Object Reference") (OtherBodyIndex :type Integer) (bFromSweep :type Boolean) (SweepResult :type "HitResult Structure (by ref)"))
  (if (== OtherActor (`GameplayStatics.GetPlayerCharacter` 0))
    (`UserWidget.AddToViewport` (`self.BadEnding`) 0)
    (set `self.InsideGood` true)))

(event `self.Bad.OnComponentEndOverlap`
  (params (OverlappedComponent :type "PrimitiveComponent Object Reference") (OtherActor :type "Actor Object Reference") (OtherComp :type "PrimitiveComponent Object Reference") (OtherBodyIndex :type Integer))
  (if (== OtherActor (`GameplayStatics.GetPlayerCharacter` 0))
    (`Widget.RemoveFromParent` (`self.BadEnding`))
    (set `self.InsideGood` false)))

(event `self.Good.OnComponentBeginOverlap`
  (params (OverlappedComponent :type "PrimitiveComponent Object Reference") (OtherActor :type "Actor Object Reference") (OtherComp :type "PrimitiveComponent Object Reference") (OtherBodyIndex :type Integer) (bFromSweep :type Boolean) (SweepResult :type "HitResult Structure (by ref)"))
  (if (== OtherActor (`GameplayStatics.GetPlayerCharacter` 0))
    (`UserWidget.AddToViewport` (`self.GoodEnding`) 0)
    (set `self.InsideBad` true)))

(event `self.Good.OnComponentEndOverlap`
  (params (OverlappedComponent :type "PrimitiveComponent Object Reference") (OtherActor :type "Actor Object Reference") (OtherComp :type "PrimitiveComponent Object Reference") (OtherBodyIndex :type Integer))
  (if (== OtherActor (`GameplayStatics.GetPlayerCharacter` 0))
    (`Widget.RemoveFromParent` (`self.GoodEnding`))
    (set `self.InsideBad` false)))

(event `self.ReceiveTick`
  (params (DeltaSeconds :type "Float (single-precision)"))
  (if (`self.PressingToEnd`)
    (if (`self.InsideBad`)
      (`PlayerCameraManager.StartCameraFade` (`GameplayStatics.GetPlayerCameraManager` 0) 0.0 1.0 3.0 (struct :`R` 1.0 :`G` 1.0 :`B` 1.0 :`A` 1.0) false false)
      (`KismetSystemLibrary.Delay` 3.0 :!label _label)
      (`GameplayStatics.OpenLevel` "MainMenuMap")
      (elif (`self.InsideGood`)
        (`PlayerCameraManager.StartCameraFade` (`GameplayStatics.GetPlayerCameraManager` 0) 0.0 1.0 3.0 (struct :`A` 1.0) false false)
        (goto _label)))))

(fn `UserConstructionScript`)